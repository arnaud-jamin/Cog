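; BP_Character is a shared character Blueprint that manages a status widget attached to the character through a widget component.
; On BeginPlay, outside dedicated servers, it binds to OnInitialized and caches the component's widget as a WBP_Status.
; When OnInitialized fires, it initializes that widget with itself and refreshes its visibility.
; SetIsTargetedByPlayer forwards the player's targeting state to the widget.
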(event Custom|On%20Initialized
  (params (Character :type Cog%20Sample%20Character%20Object%20Reference))
  (Default|Initialize (Variables|Default|GetStatusWidget) self)
  (Default|RefreshVisibility (Variables|Default|GetStatusWidget)))

(event EventBeginPlay
  (|CallParentFunction)
  (if (not (Networking|IsDedicatedServer))
    (EventDispatchers|BindEventtoOnInitialized (EventDispatchers|CreateEvent :!event Custom|On%20Initialized))
    (bind _aswbp_status (Utilities|Casting|CastToWBP_Status (UserInterface|GetWidget (Variables|Default|GetStatusWidgetComponent))))
    (Variables|Default|SetStatusWidget _aswbp_status)))

(fn ConstructionScript)

(fn SetIsTargetedbyPlayer
  (params (Value :type Boolean))
  (Default|SetIsTargeted (Variables|Default|GetStatusWidget) Value))