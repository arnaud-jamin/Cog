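; Debug cheat that teleports the target actors to the point the first player's camera is aiming at.
; Execute runs a Visibility line trace from the camera location along its forward vector, out to a fixed range.
; Every target is moved to the same hit location with a non-swept teleport, without checking whether the trace hit anything.
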(fn Execute
  (params (WorldContextObject :type Object%20Object%20Reference) (Instigator :type Actor%20Object%20Reference) (Targets :type Array%20of%20Actor%20Object%20References))
  (LocalVariables|SetCameraManager (Game|GetPlayerCameraManager WorldContextObject))
  (LocalVariables|SetTraceStartLocation (Camera|GetCameraLocation (LocalVariables|GetCameraManager)))
  (LocalVariables|SetTraceEndLocation (+ (LocalVariables|GetTraceStartLocation) (* (Math|Vector|GetForwardVector (Camera|GetCameraRotation (LocalVariables|GetCameraManager))) 1e+04)))
  (bind _outhit (Collision|LineTraceByChannel WorldContextObject (LocalVariables|GetTraceStartLocation) (LocalVariables|GetTraceEndLocation) "TraceTypeQuery1" false 0 "None"))
  (LocalVariables|SetLocation (.Location (Collision|BreakHitResult _outhit)))
  (for _array_element Targets
    (Transformation|SetActorLocation _array_element (LocalVariables|GetLocation) false true))
  (return))