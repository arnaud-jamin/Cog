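; Player controller that links the locally controlled character to the HUD and tracks which character the player targets.
; On BeginPlay, only for the local controller, it binds target and controlled-character change events and checks the possessed character.
; It initializes BP_Hud once that character is initialized, waiting on its initialization event if needed.
; Target changes move the targeted-by-player flag from the old character to the new one.
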(event EventBeginPlay
  (if (Pawn|IsLocalController)
    (EventDispatchers|BindEventtoOnTargetChanged (EventDispatchers|CreateEvent :!event OnTargetChanged))
    (EventDispatchers|BindEventtoOnControlledCharacterChanged (EventDispatchers|CreateEvent :!event WaitforPossessedCharacterInitialization))
    (CallFunction|WaitforPossessedCharacterInitialization self (Variables|Default|GetPossessedCharacter))))

(fn ConstructionScript)

(fn WaitforPossessedCharacterInitialization
  (params (Controller :type Cog%20Sample%20Player%20Controller%20Object%20Reference) (NewCharacter :type Cog%20Sample%20Character%20Object%20Reference) (OldCharacter :type Cog%20Sample%20Character%20Object%20Reference))
  (Utilities|FlowControl|Sequence
    (:then_0
      (Utilities|IsValid OldCharacter
        (:Is%20Valid
          (EventDispatchers|UnbindEventfromOnInitialized OldCharacter (EventDispatchers|CreateEvent :!event OnPossessedCharacterInitialized)))))
    (:then_1
      (Utilities|IsValid NewCharacter
        (:Is%20Valid
          (if (Class|CogSampleCharacter|IsInitialized NewCharacter)
            (CallFunction|OnPossessedCharacterInitialized NewCharacter)
            (else
              (EventDispatchers|BindEventtoOnInitialized NewCharacter (EventDispatchers|CreateEvent :!event OnPossessedCharacterInitialized)))))))))

(fn OnPossessedCharacterChanged
  (params (Controller :type Cog%20Sample%20Player%20Controller%20Object%20Reference) (Character :type Cog%20Sample%20Character%20Object%20Reference)))

(fn OnPossessedCharacterInitialized
  (params (Character :type Cog%20Sample%20Character%20Object%20Reference))
  (bind _asbp_hud (Utilities|Casting|CastToBP_Hud (HUD|GetHUD)))
  (Default|Initialize _asbp_hud Character))

(fn OnTargetChanged
  (params (Controller :type Cog%20Sample%20Player%20Controller%20Object%20Reference) (NewTarget :type Actor%20Object%20Reference) (OldTarget :type Actor%20Object%20Reference))
  (Utilities|FlowControl|Sequence
    (:then_0
      (bind _asbp_character (Utilities|Casting|CastToBP_Character OldTarget))
      (Default|SetIsTargetedbyPlayer _asbp_character false))
    (:then_1
      (bind _asbp_character_2 (Utilities|Casting|CastToBP_Character NewTarget))
      (Default|SetIsTargetedbyPlayer _asbp_character_2 true))))