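; Base projectile launcher actor that repeatedly fires projectiles of a configurable class from its Arrow component while active.
; The construction script sets the tick interval to Rate, so Tick serves as the fire timer.
; Each tick, only the authority spawns the projectile, then sets its CogSampleProjectileComponent's velocity along the projectile's forward vector, applies gravity scale and activates it.
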(event EventBeginPlay)

(event Collision|EventActorBeginOverlap
  (params (OtherActor :type Actor%20Object%20Reference)))

(event EventTick
  (params (DeltaSeconds :type Float%20%28single-precision%29))
  (if (Variables|Default|GetIsActive)
    (Networking|SwitchHasAuthority
      (:Authority
        (bind _returnvalue (Game|SpawnActorfromClass (Variables|Default|GetProjectileClass) (Transformation|GetWorldTransform (Variables|Default|GetArrow)) "AlwaysSpawn" 0 0 0 0 0))
        (Variables|Default|SetProjectile (Actor|GetComponentbyClass _returnvalue "/Script/CogSample.CogSampleProjectileComponent"))
        (Variables|/Script/Engine.MovementComponent|SetVelocity (Variables|Default|GetProjectile) (* (Transformation|GetActorForwardVector (Components|GetOwner (Variables|Default|GetProjectile))) (Variables|Default|GetProjectileSpeed)))
        (Variables|/Script/Engine.ProjectileMovementComponent|SetProjectileGravityScale (Variables|Default|GetProjectile) (Variables|Default|GetProjectileGravityScale))
        (Components|Activation|Activate (Variables|Default|GetProjectile) false)))))

(fn ConstructionScript
  (Actor|Tick|SetActorTickInterval (Variables|Default|GetRate)))